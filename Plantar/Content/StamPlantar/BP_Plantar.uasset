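; Player character for StamPlantar, with camera-relative movement, planting in place and seed throwing toward the cursor, tracked by an aim hint.
; Planting flags lock movement and further actions, and SeedEffect overlaps block planting.
; BeginPlay creates HUD and minimap, counts enemies outside Level3 and applies saved volume.
; It also handles damage with brief invincibility and camera shake, Killzone respawn, pause menu and completion screen when no enemies remain.
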(event OnComponentBeginOverlap(CapsuleComponent)
  (params (OverlappedComponent :type Primitive%20Component%20Object%20Reference) (OtherActor :type Actor%20Object%20Reference) (OtherComp :type Primitive%20Component%20Object%20Reference) (OtherBodyIndex :type Integer) (bFromSweep :type Boolean) (SweepResult :type Hit%20Result%20Structure%20%28by%20ref%29))
  (if (Actor|ActorHasTag OtherActor "SeedEffect")
    (Variables|Default|SetCannotPlantSeedHere true)
    (Development|PrintString "No plant")))

(event OnComponentEndOverlap(CapsuleComponent)
  (params (OverlappedComponent :type Primitive%20Component%20Object%20Reference) (OtherActor :type Actor%20Object%20Reference) (OtherComp :type Primitive%20Component%20Object%20Reference) (OtherBodyIndex :type Integer))
  (if (Actor|ActorHasTag OtherActor "SeedEffect")
    (Variables|Default|SetCannotPlantSeedHere false)
    (Development|PrintString "Can plant")))

(event Custom|SpawnPlant
  ;[0.03305 0.3531 0.106 0.5] Type plant
  (Game|SpawnActorfromClass "/Game/PlantsAndSeeds/Plant.Plant_C" (Math|Transform|MakeTransform (Transformation|GetWorldLocation (Variables|Default|GetSeedSpawn))) "Undefined" "MultiplyWithRoot" 0 0))

(event Custom|UpdateHinter
  (Transformation|SetWorldLocation (Variables|Default|GetHintAim) (.Location (Collision|BreakHitResult (.HitResult (Game|Player|GetHitResultUnderCursorbyChannel (Game|GetPlayerController 0) "TraceTypeQuery1" true)))) false false))

(event Custom|CheckIfComplete
  (if (<= (Variables|Default|GetEnemiesLeft) 0)
    (Game|SetGamePaused true)
    (bind _returnvalue (UserInterface|CreateWidget "/Game/UI/W_Complete.W_Complete_C"))
    (UserInterface|Viewport|AddtoViewport _returnvalue 0)))

(event Input|EnhancedActionEvents|EnhancedInputActionIA_Move
  (params (ActionValue :type Vector%202D%20Structure) (ElapsedSeconds :type Float%20%28double-precision%29) (TriggeredSeconds :type Float%20%28double-precision%29) (InputAction :type Input%20Action%20Object%20Reference :default "/Game/TopDown/Input/IA_Move.IA_Move"))
  (bind (_x _y) (Math|Vector2D|BreakVector2D ActionValue))
  (bind _camera (Variables|Camera|GetCamera))
  (bind _returnvalue (Transformation|GetWorldRotation _camera))
  (bind _yaw (Math|Rotator|BreakRotator _returnvalue))
  (bind _returnvalue_2 (Math|Rotator|MakeRotator 0.0 0.0 _yaw))
  ;[0 0.15 0.01859 0.5] Movement
  (:Triggered
    (if (and (== (Variables|Default|GetIsPlanting) false) (== (Variables|Default|GetMadePlantingAction) false))
      (if (or (== (> (Math|Float|Absolute(Float) _x) 0.5) true) (== (> (Math|Float|Absolute(Float) _y) 0.5) true))
        (Pawn|Input|AddMovementInput (Math|Vector|GetForwardVector _returnvalue_2) _y false)
        (Pawn|Input|AddMovementInput (Math|Vector|GetRightVector _returnvalue_2) _x false))))
  (:Started
    (Variables|Default|SetIsWalking true))
  (:Completed
    (Variables|Default|SetIsWalking false)))

(event Collision|EventHit
  (params (MyComp :type Primitive%20Component%20Object%20Reference) (Other :type Actor%20Object%20Reference) (OtherComp :type Primitive%20Component%20Object%20Reference) (bSelfMoved :type Boolean) (HitLocation :type Vector :default "0, 0, 0") (HitNormal :type Vector :default "0, 0, 0") (NormalImpulse :type Vector :default "0, 0, 0") (Hit :type Hit%20Result%20Structure%20%28by%20ref%29))
  (Utilities|Casting|CastToKillzone Other)
  (Transformation|SetActorLocation (Variables|Default|GetSpawnPoint) false false))

(event EventBeginPlay
  (bind _maxhealth (Variables|Default|GetMaxHealth))
  (Utilities|FlowControl|Sequence
    (:then_0
      ;[0.15 0.15 0.15 0.5] Health Bar
      (bind _returnvalue (UserInterface|CreateWidget "/Game/UI/W_UI.W_UI_C"))
      (bind _output_get (Variables|Default|SetW_HUD _returnvalue))
      (UserInterface|Viewport|AddtoViewport _output_get 0)
      (bind _output_get_2 (Variables|Default|SetCurrentHealth _maxhealth))
      (Default|SetHealth (Variables|Default|GetW_HUD) _output_get_2 _maxhealth))
    (:then_1
      (Variables|Default|SetSpawnPoint (Transformation|GetActorLocation)))
    (:then_2
      (bind _returnvalue_2 (Game|GetCurrentLevelName true))
      (if (Utilities|Enum|Equal(Enum) _returnvalue_2 "Level3")
        (Variables|/Game/UI/W_UI.W_UI_C|SetHideEnemyUI (Variables|Default|GetW_HUD) true)
        (Default|EnemyUIVisibility (Variables|Default|GetW_HUD))
        (else
          (bind _outactors (Actor|GetAllActorsOfClass "/Game/Pollution/KillableEnemy.KillableEnemy_C"))
          (Variables|Default|SetTotalEnemies (Utilities|Array|Length _outactors))
          (Variables|Default|SetEnemiesLeft (Utilities|Array|Length _outactors))
          (Variables|/Game/UI/W_UI.W_UI_C|SetHideEnemyUI (Variables|Default|GetW_HUD) false)
          (Default|EnemyUIVisibility (Variables|Default|GetW_HUD)))))
    (:then_3
      (bind _returnvalue_3 (UserInterface|CreateWidget "/Game/MiniMap/WB_MiniMap.WB_MiniMap_C"))
      (UserInterface|Viewport|AddtoViewport _returnvalue_3 0))
    (:then_4
      (bind _returnvalue_4 (SaveGame|DoesSaveGameExist "SG_Settings"))
      (if _returnvalue_4
        (bind _returnvalue_5 (SaveGame|LoadGamefromSlot "SG_Settings"))
        (bind _assg_settings (Utilities|Casting|CastToSG_Settings _returnvalue_5))
        (Audio|SetSoundMixClassOverride "/Game/Music/MasterVolume.MasterVolume" "/Game/Music/MasterSound.MasterSound" (Variables|/Game/Music/SG_Settings.SG_Settings_C|GetMasterVolume _assg_settings) 1.0 1.0 true)
        (Audio|PushSoundMixModifier "/Game/Music/MasterVolume.MasterVolume")))))

(event EventTick
  (params (DeltaSeconds :type Float%20%28single-precision%29))
  (CallFunction|UpdateHinter))

(event Game|Damage|EventAnyDamage
  (params (Damage :type Float%20%28single-precision%29) (DamageType :type Damage%20Type%20Object%20Reference) (InstigatedBy :type Controller%20Object%20Reference) (DamageCauser :type Actor%20Object%20Reference))
  ;[0.15 0.15 0.15 0.5] Take Damage
  (if (not (Variables|Default|GetIsInvincible))
    (Variables|Default|SetIsInvincible true)
    (Utilities|FlowControl|Sequence
      (:then_0
        (bind _asplayer_controller (Utilities|Casting|CastToPlayerController (Pawn|GetController)))
        (Game|Feedback|ClientStartCameraShake _asplayer_controller "/Game/StamPlantar/BP_CameraShake.BP_CameraShake_C" 1.0 "World" "0, 0, 0"))
      (:then_1
        (Variables|Default|SetCurrentHealth (Math|Integer|Max(Integer) (- (Variables|Default|GetCurrentHealth) 1)))
        (Default|SetHealth (Variables|Default|GetW_HUD) (Variables|Default|GetCurrentHealth) (Variables|Default|GetMaxHealth)))
      (:then_2
        (Utilities|FlowControl|Delay 1.0)
        (Variables|Default|SetIsInvincible false)))))

(event Input|KeyboardEvents|SpaceBar
  (params (Key :type Key%20Structure :default "None"))
  ;[0.1375 0.4323 0.2116 0.5] If walking, throw seed, if not, plant normally
  (:Pressed
    (if (not (Variables|Default|GetMadePlantingAction))
      (if (not (Variables|Default|GetCannotPlantSeedHere))
        (Variables|Default|SetIsPlanting true)
        (Variables|Default|SetMadePlantingAction true)))))

(event Input|KeyboardEvents|1
  (params (Key :type Key%20Structure :default "None"))
  (:Pressed
    (bind _returnvalue (Actor|GetActorOfClass "/Game/Prefabs/TemporaryLevelSpawn.TemporaryLevelSpawn_C"))
    (Transformation|SetActorLocation (Transformation|GetActorLocation _returnvalue) false false)))

(event Input|MouseEvents|LeftMouseButton
  (params (Key :type Key%20Structure :default "None"))
  (bind _seedspawn1 (Variables|Default|GetSeedSpawn1))
  (:Pressed
    (if (not (Variables|Default|GetMadePlantingAction))
      (Variables|Default|SetIsThrowing true)
      (Transformation|SetActorRotation (Math|Rotator|FindLookatRotation (Transformation|GetActorLocation) (.Location (Collision|BreakHitResult (.HitResult (Game|Player|GetHitResultUnderCursorbyChannel (Game|GetPlayerController 0) "TraceTypeQuery1" true))))))
      (Game|SpawnActorfromClass "/Game/PlantsAndSeeds/Seed.Seed_C" (Math|Transform|MakeTransform (Transformation|GetWorldLocation _seedspawn1) (Transformation|GetWorldRotation _seedspawn1)) "Undefined" "MultiplyWithRoot" 0 0)
      (Variables|Default|SetMadePlantingAction true))))

(event Input|KeyboardEvents|Escape
  (params (Key :type Key%20Structure :default "None"))
  ;[0.15 0.15 0.15 0.5] Pause Menu
  (:Pressed
    (if (Variables|Default|GetIsPauseMenuOpen)
      (Variables|Default|SetIsPauseMenuOpen false)
      (Widget|RemovefromParent (Variables|Default|GetPauseMenuWidget))
      (Game|SetGamePaused false)
      (else
        (Variables|Default|SetIsPauseMenuOpen true)
        (bind _returnvalue (UserInterface|CreateWidget "/Game/UI/W_PauseMenu.W_PauseMenu_C" (Game|GetPlayerController 0)))
        (bind _output_get (Variables|Default|SetPauseMenuWidget _returnvalue))
        (UserInterface|Viewport|AddtoViewport (Variables|Default|GetPauseMenuWidget) 0)
        (Game|SetGamePaused true)))))

(fn ConstructionScript)