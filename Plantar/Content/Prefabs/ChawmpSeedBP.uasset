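; ChawmpSeedBP is an actor that lunges at Seed actors entering its Sight component, destroys them, then returns to its starting spot.
; Tick switches between hunting, a brief eating pause and a slower return home, using Eating and ReturnHome flags.
; A shared MoveTowardsObject event turns the ChawmpSeed component toward its goal and advances it along local axes without sweeping.
; If the target vanishes mid-chase, it still pauses and returns home.
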(event OnComponentBeginOverlap(Sight)
  (params (OverlappedComponent :type Primitive%20Component%20Object%20Reference) (OtherActor :type Actor%20Object%20Reference) (OtherComp :type Primitive%20Component%20Object%20Reference) (OtherBodyIndex :type Integer) (bFromSweep :type Boolean) (SweepResult :type Hit%20Result%20Structure%20%28by%20ref%29))
  (bind _asseed (Utilities|Casting|CastToSeed OtherActor))
  (Variables|Default|SetTargetSeed _asseed))

(event Custom|HuntDownSeed
  (bind _targetseed (Variables|Default|GetTargetSeed))
  (bind _hitbox (Variables|/Game/PlantsAndSeeds/Seed.Seed_C|GetHitbox _targetseed))
  (bind _returnvalue (Transformation|GetWorldLocation _hitbox))
  (if (Utilities|IsValid _targetseed)
    (Variables|Default|SetChaseSeed true)
    (Variables|Default|SetSeedDidSpot true)
    (CallFunction|MoveTowardsObject _returnvalue "4000.000000,0.000000,0.000000")
    (if (< (Class|KismetMathLibrary|VectorDistanceSquared (Transformation|GetWorldLocation (Variables|Default|GetChawmp_Seed)) _returnvalue) 1e+03)
      (Variables|Default|SetEating true)
      (Actor|DestroyActor (Variables|Default|GetTargetSeed)))
    (else
      (Variables|Default|SetChaseSeed false)
      (if (Variables|Default|GetSeedDidSpot)
        (Variables|Default|SetEating true)))))

(event Custom|MoveTowardsObject
  (params (TargetLocation :type Vector) (Speed :type Vector))
  (bind _chawmp_seed (Variables|Default|GetChawmp_Seed))
  (Transformation|SetWorldRotation _chawmp_seed (Math|Rotator|FindLookatRotation (Transformation|GetWorldLocation _chawmp_seed) TargetLocation) false false)
  (Transformation|AddLocalOffset _chawmp_seed (* Speed (Utilities|Time|GetWorldDeltaSeconds)) false false))

(event EventBeginPlay
  (bind _chawmp_seed (Variables|Default|GetChawmp_Seed))
  (Variables|Default|SetOrigin (Transformation|GetWorldLocation _chawmp_seed))
  (Variables|Default|SetOriginalRotate (Transformation|GetWorldRotation _chawmp_seed)))

(event EventTick
  (params (DeltaSeconds :type Float%20%28single-precision%29))
  (if (Variables|Default|GetEating)
    (if (Variables|Default|GetReturnHome)
      (CallFunction|MoveTowardsObject (Variables|Default|GetOrigin) "800.000000,0.000000,0.000000")
      (if (< (Class|KismetMathLibrary|VectorDistanceSquared (Transformation|GetWorldLocation (Variables|Default|GetChawmp_Seed)) (Variables|Default|GetOrigin)) 5e+01)
        (Variables|Default|SetEating false)
        (Variables|Default|SetReturnHome false)
        (Transformation|SetWorldRotation (Variables|Default|GetChawmp_Seed) (Variables|Default|GetOriginalRotate) false false)
        (Variables|Default|SetTargetSeed 0)
        (Variables|Default|SetSeedDidSpot false))
      (else
        (Utilities|FlowControl|Delay 0.5)
        (Variables|Default|SetReturnHome true)))
    (else
      (CallFunction|HuntDownSeed))))

(fn ConstructionScript)