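; Fumer Blueprint that detects when exported Niagara particles land near plantar objects, likely for a fertilizing mechanic still at the debug stage.
; On BeginPlay it caches the BP_Plantar actor and registers itself as the Niagara UserCallback for particle data export.
; Each received particle position gets a sphere trace, and a hit component whose display name contains "Plantar" currently only prints a debug message.
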(event EventParticleData
  (params (Data :type Array%20of%20Basic%20Particle%20Data%20Structures) (NiagaraSystem :type Niagara%20System%20Object%20Reference) (SimulationPositionOffset :type Vector%20%28by%20ref%29 :default "0, 0, 0"))
  (for _array_element Data
    (bind _outhit (Collision|SphereTraceByChannel (.Position (Utilities|Struct|BreakBasicParticleData _array_element)) (.Position (Utilities|Struct|BreakBasicParticleData _array_element)) 1.8e+02 "TraceTypeQuery1" false 0 "None"))
    (if (Utilities|String|Contains (Utilities|GetDisplayName (.HitComponent (Collision|BreakHitResult _outhit))) "Plantar")
      (Development|PrintString "Hello"))))

(event EventBeginPlay
  (bind _returnvalue (Actor|GetActorOfClass "/Game/StamPlantar/BP_Plantar.BP_Plantar_C"))
  (Variables|Default|SetPlantar _returnvalue)
  (Class|NiagaraComponent|SetVariableObject (Variables|Default|GetNiagara) "UserCallback" self))

(fn ConstructionScript)