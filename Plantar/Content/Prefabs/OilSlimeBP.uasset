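; Oil slime enemy that chases BP_Plantar, damages it on attack-hitbox overlap, and splits when hit by harmful plants.
; While ticking, it applies size, speed and animation rate from its shrink tier, moves toward the player and, if shrunk, hops at random intervals.
; After brief spawn immunity, a harmful Plant overlap spawns two next-tier copies and destroys the original.
; The final tier or a Killzone hit destroys it.
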(event OnComponentBeginOverlap(Box)
  (params (OverlappedComponent :type Primitive%20Component%20Object%20Reference) (OtherActor :type Actor%20Object%20Reference) (OtherComp :type Primitive%20Component%20Object%20Reference) (OtherBodyIndex :type Integer) (bFromSweep :type Boolean) (SweepResult :type Hit%20Result%20Structure%20%28by%20ref%29))
  (bind _box (Variables|Default|GetBox))
  (bind _asplant (Utilities|Casting|CastToPlant OtherActor))
  (if (Math|Boolean|ANDBoolean (== (Variables|/Game/PlantsAndSeeds/Plant.Plant_C|GetHarmfulTime _asplant) true) (== (Variables|Default|GetImmunity) false) (== (Variables|Default|GetSplit) false))
    (for _index (range 0 1)
      (bind _returnvalue (Game|SpawnActorfromClass "OilSlimeBP_C" (Math|Transform|MakeTransform (Transformation|GetWorldLocation _box) (Transformation|GetWorldRotation _box)) "AdjustIfPossibleButAlwaysSpawn" "MultiplyWithRoot" 0 0))
      (Variables|Default|SetIsClone true)
      (Variables|OilSlimeBP_C|SetSizeShrink _returnvalue (+ (Variables|Default|GetSizeShrink) 1))
      (Transformation|AddLocalOffset _box "10.000000,0.000000,0.000000" false false))
    (Variables|Default|SetSplit true)
    (Actor|DestroyActor)))

(event OnComponentHit(Box)
  (params (HitComponent :type Primitive%20Component%20Object%20Reference) (OtherActor :type Actor%20Object%20Reference) (OtherComp :type Primitive%20Component%20Object%20Reference) (NormalImpulse :type Vector :default "0, 0, 0") (Hit :type Hit%20Result%20Structure%20%28by%20ref%29))
  (Utilities|Casting|CastToKillzone OtherActor)
  (Actor|DestroyActor))

(event OnComponentBeginOverlap(AttackHitBox)
  (params (OverlappedComponent :type Primitive%20Component%20Object%20Reference) (OtherActor :type Actor%20Object%20Reference) (OtherComp :type Primitive%20Component%20Object%20Reference) (OtherBodyIndex :type Integer) (bFromSweep :type Boolean) (SweepResult :type Hit%20Result%20Structure%20%28by%20ref%29))
  ;[0.15 0.15 0.15 0.5] Damage Player
  (bind _asbp_plantar (Utilities|Casting|CastToBP_Plantar OtherActor))
  (Game|Damage|ApplyDamage _asbp_plantar 1.0 0 0))

(event Custom|SizeMake
  (switch int (Variables|Default|GetSizeShrink)
    (:0
      (Variables|Default|SetSizer 5.0)
      (Variables|Default|SetSpeed 5e+01)
      (Variables|Default|SetAnimSpeed 1.0)
      (Transformation|SetRelativeScale3D (Variables|Default|GetBox) (Math|Vector|MakeVector (Variables|Default|GetSizer) (Variables|Default|GetSizer) (Variables|Default|GetSizer)) :!label _label)
      (Components|Timeline|SetPlayRate (Variables|Default|GetSkeletalMesh) (Variables|Default|GetAnimSpeed)))
    (:1
      (Variables|Default|SetSizer 3.0)
      (Variables|Default|SetSpeed 1e+02)
      (Variables|Default|SetAnimSpeed 2.0)
      (goto _label))
    (:2
      (Variables|Default|SetSizer 1.5)
      (Variables|Default|SetSpeed 2e+02)
      (Variables|Default|SetAnimSpeed 3.0)
      (goto _label))
    (:3
      (Variables|Default|SetSizer 1.0)
      (Variables|Default|SetSpeed 3.5e+02)
      (Variables|Default|SetAnimSpeed 6.0)
      (goto _label))
    (:4
      (Actor|DestroyActor))))

(event Custom|Chase
  (bind _box (Variables|Default|GetBox))
  (if (Utilities|IsValid _box)
    (Transformation|SetWorldRotation _box (Math|Rotator|MakeRotator 0.0 0.0 (.Yaw (Math|Rotator|BreakRotator (Math|Rotator|FindLookatRotation (Transformation|GetWorldLocation _box) (Transformation|GetActorLocation (Variables|Default|GetPlantar)))))) false false)
    (Transformation|AddLocalOffset _box (* (Math|Vector|MakeVector (Variables|Default|GetSpeed) 0.0 0.0) (Utilities|Time|GetWorldDeltaSeconds)) false false)))

(event Custom|Jump
  (Physics|AddImpulse (Variables|Default|GetBox) "0.000000,0.000000,24999.750000" "None" false))

(event EventTick
  (params (DeltaSeconds :type Float%20%28single-precision%29))
  (|CallParentFunction 0.0)
  (CallFunction|SizeMake)
  (CallFunction|Chase)
  (if (!= (Variables|Default|GetSizeShrink) 0)
    (Utilities|FlowControl|Delay (Math|Random|RandomFloatinRange 1.0 3.0))
    (CallFunction|Jump)))

(event EventBeginPlay
  (bind _returnvalue (Actor|GetActorOfClass "/Game/StamPlantar/BP_Plantar.BP_Plantar_C"))
  (Variables|Default|SetPlantar _returnvalue)
  (Variables|Default|SetImmunity true)
  (Utilities|FlowControl|Delay 0.5)
  (Variables|Default|SetImmunity false)
  (if (Variables|Default|GetIsClone)
    (Actor|Tick|SetActorTickEnabled true)
    (else
      (Actor|Tick|SetActorTickEnabled false))))

(fn ConstructionScript)