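; WasticBP is an enemy that homes in on BP_Plantar and deals damage when its attack hitbox overlaps it.
; BeginPlay registers itself as Child, caches the Plantar and disables tick, with no re-enable in this file.
; When ticking, it calls parent Tick, yaws its Box toward the Plantar and advances it without sweep at constant speed.
; It destroys itself on hitting a Killzone or overlapping a Plant during HarmfulTime.
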(event OnComponentBeginOverlap(Box)
  (params (OverlappedComponent :type Primitive%20Component%20Object%20Reference) (OtherActor :type Actor%20Object%20Reference) (OtherComp :type Primitive%20Component%20Object%20Reference) (OtherBodyIndex :type Integer) (bFromSweep :type Boolean) (SweepResult :type Hit%20Result%20Structure%20%28by%20ref%29))
  (bind _asplant (Utilities|Casting|CastToPlant OtherActor))
  (if (Variables|/Game/PlantsAndSeeds/Plant.Plant_C|GetHarmfulTime _asplant)
    (Actor|DestroyActor)))

(event OnComponentHit(Box)
  (params (HitComponent :type Primitive%20Component%20Object%20Reference) (OtherActor :type Actor%20Object%20Reference) (OtherComp :type Primitive%20Component%20Object%20Reference) (NormalImpulse :type Vector :default "0, 0, 0") (Hit :type Hit%20Result%20Structure%20%28by%20ref%29))
  (Utilities|Casting|CastToKillzone OtherActor)
  (Actor|DestroyActor))

(event OnComponentBeginOverlap(AttackHitBox)
  (params (OverlappedComponent :type Primitive%20Component%20Object%20Reference) (OtherActor :type Actor%20Object%20Reference) (OtherComp :type Primitive%20Component%20Object%20Reference) (OtherBodyIndex :type Integer) (bFromSweep :type Boolean) (SweepResult :type Hit%20Result%20Structure%20%28by%20ref%29))
  ;[0.15 0.15 0.15 0.5] Damage Player
  (bind _asbp_plantar (Utilities|Casting|CastToBP_Plantar OtherActor))
  (Game|Damage|ApplyDamage _asbp_plantar 1.0 0 0))

(event EventBeginPlay
  (Variables|Default|SetChild self)
  (bind _returnvalue (Actor|GetActorOfClass "/Game/StamPlantar/BP_Plantar.BP_Plantar_C"))
  (Variables|Default|SetPlantar _returnvalue)
  (Actor|Tick|SetActorTickEnabled false))

(event EventTick
  (params (DeltaSeconds :type Float%20%28single-precision%29))
  (bind _box (Variables|Default|GetBox))
  (|CallParentFunction 0.0)
  (Transformation|SetWorldRotation _box (Math|Rotator|MakeRotator 0.0 0.0 (.Yaw (Math|Rotator|BreakRotator (Math|Rotator|FindLookatRotation (Transformation|GetWorldLocation _box) (Transformation|GetActorLocation (Variables|Default|GetPlantar)))))) false false)
  (Transformation|AddLocalOffset _box (* "200.000000,0.000000,0.000000" (Utilities|Time|GetWorldDeltaSeconds)) false false))

(fn ConstructionScript)